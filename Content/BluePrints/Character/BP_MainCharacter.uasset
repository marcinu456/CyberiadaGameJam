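; Player character Blueprint that handles movement, a mask toggle, item pickup input and pausing.
; BeginPlay adds the default Enhanced Input context and enables Game and UI input with a visible cursor.
; Mask toggling is gated by CanMask and, like the get-item input, broadcasts through event dispatchers; pause creates a menu widget and pauses the game.
; Getter functions expose the character and BP_GameHud.
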(event `self.ReceiveBeginPlay`
  (bind _returnvalue (`GameplayStatics.GetPlayerController` 0))
  (bind _asplayer_controller (cast `PlayerController` (`self.GetController`)))
  (`EnhancedInputSubsystemInterface.AddMappingContext` (pcsubsystem `EnhancedInputLocalPlayerSubsystem` _asplayer_controller) "/Game/BluePrints/Character/InputAction/IMC_Default.IMC_Default" 0 (struct))
  (`WidgetBlueprintLibrary.SetInputMode_GameAndUIEx` _returnvalue null)
  (set `PlayerController.bShowMouseCursor` true _returnvalue))

(event `EnhancedInput|/Game/BluePrints/Character/InputAction/IA_Movement`
  (params (ActionValue :type "Vector2D Structure") (ElapsedSeconds :type "Float (double-precision)") (TriggeredSeconds :type "Float (double-precision)") (InputAction :type "InputAction Object Reference" :default "/Game/BluePrints/Character/InputAction/IA_Movement.IA_Movement"))
  (:`Triggered`
    (`self.AddMovementInput` (`self.GetActorForwardVector`) ActionValue_X)
    (`self.AddMovementInput` (`self.GetActorRightVector`) ActionValue_Y)
    (set `self.IsWalkingRight` (>= ActionValue_X 0.1))))

(event `EnhancedInput|/Game/BluePrints/Character/InputAction/IA_ChangeMask`
  (params (ActionValue :type Boolean) (ElapsedSeconds :type "Float (double-precision)") (TriggeredSeconds :type "Float (double-precision)") (InputAction :type "InputAction Object Reference" :default "/Game/BluePrints/Character/InputAction/IA_ChangeMask.IA_ChangeMask"))
  (:`Triggered`
    (if (`self.CanMask`)
      (if (`self.Mask`)
        (set `self.Mask` false)
        (`KismetSystemLibrary.PrintString` "Off")
        (`self.ED_CurrentMaskStatus` false)
        (else
          (set `self.Mask` true)
          (`KismetSystemLibrary.PrintString` "On")
          (`self.ED_CurrentMaskStatus` true)))
      (else
        (`KismetSystemLibrary.PrintString` "nie mas zmaski")))))

(event `EnhancedInput|/Game/BluePrints/Character/InputAction/IA_Pause`
  (params (ActionValue :type Boolean) (ElapsedSeconds :type "Float (double-precision)") (TriggeredSeconds :type "Float (double-precision)") (InputAction :type "InputAction Object Reference" :default "/Game/BluePrints/Character/InputAction/IA_Pause.IA_Pause"))
  (:`Started`
    (bind _returnvalue (`|CreateWidget` "/Game/Widgets/PuaseMenu/WBP_PauseMenu.WBP_PauseMenu_C" (`GameplayStatics.GetPlayerController` 0)))
    (bind _output_get (set `self.PauseMenuWidget` _returnvalue))
    (`UserWidget.AddToViewport` _output_get 0)
    (`GameplayStatics.SetGamePaused` true)))

(event `EnhancedInput|/Game/BluePrints/Character/InputAction/IA_GetItem`
  (params (ActionValue :type Boolean) (ElapsedSeconds :type "Float (double-precision)") (TriggeredSeconds :type "Float (double-precision)") (InputAction :type "InputAction Object Reference" :default "/Game/BluePrints/Character/InputAction/IA_GetItem.IA_GetItem"))
  (:`Started`
    (`self.ED_GetItem`)))

(fn `Get_BPMainCharacter`
  (returns (BPMainCharacterOut :type "/Game/BluePrints/Character/BP_MainCharacter Soft Object Reference"))
  (return (`|ConvertAsset` self)))

(fn `GetBPGameHud`
  (returns (GameHUD :type "/Game/BluePrints/UI/BP_GameHud Object Reference"))
  (bind _asbp_game_hud (cast `/Game/BluePrints/UI/BP_GameHud` (`PlayerController.GetHUD` (`GameplayStatics.GetPlayerController` 0))))
  (return _asbp_game_hud))

(fn `UserConstructionScript`)