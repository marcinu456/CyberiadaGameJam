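; Base sprite interact actor for item pickups, shown or hidden according to the player's mask state.
; While active, box overlap tints the sprite and binds to the character's get-item dispatcher, unbinding on exit.
; That event adds the item's DT_Items row to the inventory and disables the box.
; Visibility follows per-mask-state flags, and helpers add or remove HUD widgets for derived actors.
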(event `self.ReceiveBeginPlay`
  (bind _asbp_main_character (cast `/Game/BluePrints/Character/BP_MainCharacter` (`GameplayStatics.GetPlayerCharacter` 0)))
  (bind _output_get (set `self.RefToMainCharToDest` _asbp_main_character))
  (add `/Game/BluePrints/Character/BP_MainCharacter.ED_CurrentMaskStatus` _output_get (`|CreateDelegate` :!event `SetHideInGameStatus`))
  (`self.SetHideInGameStatus` false))

(event `GiveItemToCharacter`
  (remove `/Game/BluePrints/Character/BP_MainCharacter.ED_GetItem` (stale `self.Box.OnComponentBeginOverlap` _asbp_main_character) (delegate `GiveItemToCharacter`))
  (bind _asbp_main_character (cast `/Game/BluePrints/Character/BP_MainCharacter` (`GameplayStatics.GetPlayerCharacter` 0)))
  (bind _returnvalue (`|GetDataTableRow` "/Game/BluePrints/DataTables/DT_Items.DT_Items" (`.RowName` (break `DataTableRowHandle` (`self.ItemInActor`))))
    (:`then`
      (`/Game/BluePrints/Components/Player/BP_InventoryComponents.AddItemToInv` (`/Game/BluePrints/Character/BP_MainCharacter.BP_InventoryComponents` _asbp_main_character) _returnvalue)
      (set `/Game/BluePrints/Character/BP_MainCharacter.bCanGetItem` false _asbp_main_character)
      (`PrimitiveComponent.SetCollisionEnabled` (`self.Box`) "NoCollision"))))

(event `self.Box.OnComponentBeginOverlap`
  (params (OverlappedComponent :type "PrimitiveComponent Object Reference") (OtherActor :type "Actor Object Reference") (OtherComp :type "PrimitiveComponent Object Reference") (OtherBodyIndex :type Integer) (bFromSweep :type Boolean) (SweepResult :type "HitResult Structure (by ref)"))
  (bind _rendercomponent (`self.RenderComponent`))
  (if (`self.BItemIsActive`)
    (bind _asbp_main_character (cast `/Game/BluePrints/Character/BP_MainCharacter` (`GameplayStatics.GetPlayerCharacter` 0)))
    (add `/Game/BluePrints/Character/BP_MainCharacter.ED_GetItem` _asbp_main_character (delegate `GiveItemToCharacter`))
    (set `/Game/BluePrints/Character/BP_MainCharacter.bCanGetItem` true _asbp_main_character)
    (`KismetSystemLibrary.PrintString` "OverlapInteactActor")
    (set `self.Sprite Color Backup` (`PaperSpriteComponent.SpriteColor` _rendercomponent))
    (`PaperSpriteComponent.SetSpriteColor` _rendercomponent (`self.New Color`))))

(event `self.Box.OnComponentEndOverlap`
  (params (OverlappedComponent :type "PrimitiveComponent Object Reference") (OtherActor :type "Actor Object Reference") (OtherComp :type "PrimitiveComponent Object Reference") (OtherBodyIndex :type Integer))
  (if (`self.BItemIsActive`)
    (bind _asbp_main_character (cast `/Game/BluePrints/Character/BP_MainCharacter` (`GameplayStatics.GetPlayerCharacter` 0)))
    (remove `/Game/BluePrints/Character/BP_MainCharacter.ED_GetItem` _asbp_main_character (delegate `GiveItemToCharacter`))
    (set `/Game/BluePrints/Character/BP_MainCharacter.bCanGetItem` false _asbp_main_character)
    (`KismetSystemLibrary.PrintString` "StopOverlap")
    (`PaperSpriteComponent.SetSpriteColor` (`self.RenderComponent`) (`self.Sprite Color Backup`))))

(fn `AddOrRemoveWidget`
  (params (Widget :type "UserWidget Object Reference"))
  (bind _returnvalue (`GameplayStatics.GetPlayerController` 0))
  (bind _asbp_game_hud (cast `/Game/BluePrints/UI/BP_GameHud` (`PlayerController.GetHUD` (`GameplayStatics.GetPlayerController` 0))))
  (if (not (`PanelWidget.HasChild` (`/Game/Widgets/Game/WBP_GameInterface.HideCanwas` (`/Game/BluePrints/UI/BP_GameHud.GameInterface` _asbp_game_hud)) Widget))
    (`|ExecutionSequence`
      (:`then_0`
        (`/Game/BluePrints/UI/BP_GameHud.AddWidget` _asbp_game_hud Widget)
        (`WidgetBlueprintLibrary.SetInputMode_GameAndUIEx` _returnvalue null)
        (set `PlayerController.bShowMouseCursor` true _returnvalue))
      (:`then_1`
        (`CanvasPanelSlot.SetAnchors` (`WidgetLayoutLibrary.SlotAsCanvasSlot` Widget) (make `Anchors` (0.0 0.0) (1.0 1.0)))))
    (else
      (`/Game/BluePrints/UI/BP_GameHud.RemoveWidget` _asbp_game_hud Widget))))

(fn `HideObject`
  (`SceneComponent.SetHiddenInGame` (`self.RenderComponent`) true false)
  (`PrimitiveComponent.SetCollisionEnabled` (`self.RenderComponent`) "NoCollision"))

(fn `RemoveFromGameWidget`
  (params (UserWidget :type "UserWidget Object Reference"))
  (bind _asbp_game_hud (cast `/Game/BluePrints/UI/BP_GameHud` (`PlayerController.GetHUD` (`GameplayStatics.GetPlayerController` 0))))
  (`/Game/BluePrints/UI/BP_GameHud.RemoveWidget` _asbp_game_hud UserWidget))

(fn `SetHideInGameStatus`
  (params (bWearMask :type Boolean))
  (if bWearMask
    (if (`self.bShowWhenMasked`)
      (`self.UnHideObject` :!label _label)
      (else
        (`self.HideObject` :!label _label_2)))
    (elif (`self.bShowWhenNoMasked`)
      (goto _label)
      (else
        (goto _label_2)))))

(fn `UnHideObject`
  (`SceneComponent.SetHiddenInGame` (`self.RenderComponent`) false false)
  (if (`self.BItemIsActive`)
    (`PrimitiveComponent.SetCollisionEnabled` (`self.RenderComponent`) "QueryAndPhysics")))

(fn `UserConstructionScript`)