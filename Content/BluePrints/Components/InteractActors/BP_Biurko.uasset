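; BP_Biurko is an actor (Polish for "desk") that is visible only while the player character's Mask flag is set.
; On BeginPlay it hides itself and caches player 0's pawn as BP_MainCharacter.
; Tick polls that Mask flag every frame and toggles Hidden In Game to match, without changing collision.
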(event `self.ReceiveBeginPlay`
  (`self.SetActorHiddenInGame` true)
  (bind _asbp_main_character (cast `/Game/BluePrints/Character/BP_MainCharacter` (`GameplayStatics.GetPlayerCharacter` 0)))
  (set `self.As BP Main Character` _asbp_main_character))

(event `self.ReceiveTick`
  (params (DeltaSeconds :type "Float (single-precision)"))
  (if (`/Game/BluePrints/Character/BP_MainCharacter.Mask` (`self.As BP Main Character`))
    (`self.SetActorHiddenInGame` false)
    (else
      (`self.SetActorHiddenInGame` true))))

(fn `UserConstructionScript`
  (`parent.UserConstructionScript`))