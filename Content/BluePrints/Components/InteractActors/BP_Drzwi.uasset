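; BP_Drzwi is an interactable sprite door that teleports the player to a linked door once puzzle 3 (Zagadka3Done) is solved.
; Overlapping its box tints the sprite, enables CanGetItem and binds Door to the main character's GetItem dispatcher; leaving reverses this.
; Door moves the player to DoorToNextLevel's TeleportPlace offset and switches the view to CameraToNextLevel if set.
; An unset target door only prints a setup warning.
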(event `Door`
  (bind _doortonextlevel (`self.DoorToNextLevel`)
    (:`then`
      (if (and true (`/Game/BluePrints/Character/BP_MainCharacter.Zagadka3Done` (`self.RefToMainCharToDest`)))
        (`self.K2_SetActorLocation` (`GameplayStatics.GetPlayerCharacter` 0) (+ (`self.K2_GetActorLocation` _doortonextlevel) (`SceneComponent.RelativeLocation` (`/Game/BluePrints/Components/InteractActors/BP_Drzwi.TeleportPlace` _doortonextlevel))) false true)
        (bind _cameratonextlevel (`self.CameraToNextLevel`)
          (:`then`
            (`PlayerController.SetViewTargetWithBlend` (`GameplayStatics.GetPlayerController` 0) _cameratonextlevel 0.0 "VTBlend_Linear" 0.0 false))
          (:`else`))))
    (:`else`
      (`KismetSystemLibrary.PrintString` "Setup Door"))))

(event `self.Box.OnComponentBeginOverlap`
  (params (OverlappedComponent :type "PrimitiveComponent Object Reference") (OtherActor :type "Actor Object Reference") (OtherComp :type "PrimitiveComponent Object Reference") (OtherBodyIndex :type Integer) (bFromSweep :type Boolean) (SweepResult :type "HitResult Structure (by ref)"))
  (bind _rendercomponent (`self.RenderComponent`))
  (bind _asbp_main_character (cast `/Game/BluePrints/Character/BP_MainCharacter` (`GameplayStatics.GetPlayerCharacter` 0)))
  (add `/Game/BluePrints/Character/BP_MainCharacter.ED_GetItem` _asbp_main_character (delegate `Door`))
  (set `/Game/BluePrints/Character/BP_MainCharacter.bCanGetItem` true _asbp_main_character)
  (`KismetSystemLibrary.PrintString` "OverlapKufer")
  (set `self.Sprite Color Backup` (`PaperSpriteComponent.SpriteColor` _rendercomponent))
  (`PaperSpriteComponent.SetSpriteColor` _rendercomponent (`self.New Color`)))

(event `self.Box.OnComponentEndOverlap`
  (params (OverlappedComponent :type "PrimitiveComponent Object Reference") (OtherActor :type "Actor Object Reference") (OtherComp :type "PrimitiveComponent Object Reference") (OtherBodyIndex :type Integer))
  (bind _asbp_main_character (cast `/Game/BluePrints/Character/BP_MainCharacter` (`GameplayStatics.GetPlayerCharacter` 0)))
  (remove `/Game/BluePrints/Character/BP_MainCharacter.ED_GetItem` _asbp_main_character (delegate `Door`))
  (set `/Game/BluePrints/Character/BP_MainCharacter.bCanGetItem` false _asbp_main_character)
  (`KismetSystemLibrary.PrintString` "StopOverlap")
  (`PaperSpriteComponent.SetSpriteColor` (`self.RenderComponent`) (`self.Sprite Color Backup`)))

(fn `UserConstructionScript`
  (`parent.UserConstructionScript`))