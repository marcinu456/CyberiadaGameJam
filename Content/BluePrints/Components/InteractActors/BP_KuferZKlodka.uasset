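; Padlocked chest actor that opens a lock riddle and holds the mask item for the player.
; While the player overlaps its Box, it tints the sprite and binds to the character's get-item dispatcher to toggle the WBP_Riddle2 widget, whose solved event is bound back to the chest.
; GiveMask adds the DT_Items row to inventory, enables the mask and disables the Box.
; Tick hides the sprite while Mask is set, disabling its collision without restoring it.
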(event `self.ReceiveBeginPlay`
  (`parent.ReceiveBeginPlay`)
  (bind _asbp_main_character (cast `/Game/BluePrints/Character/BP_MainCharacter` (`GameplayStatics.GetPlayerCharacter` 0)))
  (set `self.MainCharacter` _asbp_main_character))

(event `self.ReceiveTick`
  (params (DeltaSeconds :type "Float (single-precision)"))
  (if (`/Game/BluePrints/Character/BP_MainCharacter.Mask` (`self.MainCharacter`))
    (`SceneComponent.SetHiddenInGame` (`self.RenderComponent`) true false)
    (`PrimitiveComponent.SetCollisionEnabled` (`self.RenderComponent`) "NoCollision")
    (else
      (`SceneComponent.SetHiddenInGame` (`self.RenderComponent`) false false))))

(event `self.GiveItemToCharacter`
  (`self.WBP_Riddle2`
    (:`then`
      _)
    (:`else`
      (bind _returnvalue (`|CreateWidget` "/Game/Widgets/Riddle2/WBP_Riddle2.WBP_Riddle2_C" (`GameplayStatics.GetPlayerController` 0)))
      (bind _output_get (set `self.WBP_Riddle2` _returnvalue))
      (add `/Game/Widgets/Riddle2/WBP_Riddle2.ED_SolvedLock` _output_get (`|CreateDelegate` :!event `GiveMask`))))
  (`/Engine/EditorBlueprintResources/StandardMacros.FlipFlop`
    (:`A`
      _)
    (:`B`
      _))
  (`self.AddOrRemoveWidget` (`self.WBP_Riddle2`)))

(event `GiveMask`
  ; GiveMaskToPlayer
  (bind _maincharacter (`self.MainCharacter`)
    (:`then`
      (bind _returnvalue (`|GetDataTableRow` "/Game/BluePrints/DataTables/DT_Items.DT_Items" (`.RowName` (break `DataTableRowHandle` (`self.ItemInActor`))))
        (:`then`
          (`/Game/BluePrints/Components/Player/BP_InventoryComponents.AddItemToInv` (`/Game/BluePrints/Character/BP_MainCharacter.BP_InventoryComponents` _maincharacter) _returnvalue)
          (set `/Game/BluePrints/Character/BP_MainCharacter.bCanGetItem` false _maincharacter)
          (`PrimitiveComponent.SetCollisionEnabled` (`self.Box`) "NoCollision")
          (set `/Game/BluePrints/Character/BP_MainCharacter.CanMask` true _maincharacter)
          (remove `/Game/BluePrints/Character/BP_MainCharacter.ED_GetItem` (stale `self.Box.OnComponentBeginOverlap` _asbp_main_character) (delegate `self.GiveItemToCharacter`)))))
    (:`else`)))

(event `self.Box.OnComponentBeginOverlap`
  (params (OverlappedComponent :type "PrimitiveComponent Object Reference") (OtherActor :type "Actor Object Reference") (OtherComp :type "PrimitiveComponent Object Reference") (OtherBodyIndex :type Integer) (bFromSweep :type Boolean) (SweepResult :type "HitResult Structure (by ref)"))
  (bind _rendercomponent (`self.RenderComponent`))
  (bind _asbp_main_character (cast `/Game/BluePrints/Character/BP_MainCharacter` (`GameplayStatics.GetPlayerCharacter` 0)))
  (add `/Game/BluePrints/Character/BP_MainCharacter.ED_GetItem` _asbp_main_character (delegate `self.GiveItemToCharacter`))
  (set `/Game/BluePrints/Character/BP_MainCharacter.bCanGetItem` true _asbp_main_character)
  (`KismetSystemLibrary.PrintString` "OverlapKufer")
  (set `self.Sprite Color Backup` (`PaperSpriteComponent.SpriteColor` _rendercomponent))
  (`PaperSpriteComponent.SetSpriteColor` _rendercomponent (`self.New Color`)))

(event `self.Box.OnComponentEndOverlap`
  (params (OverlappedComponent :type "PrimitiveComponent Object Reference") (OtherActor :type "Actor Object Reference") (OtherComp :type "PrimitiveComponent Object Reference") (OtherBodyIndex :type Integer))
  (bind _asbp_main_character (cast `/Game/BluePrints/Character/BP_MainCharacter` (`GameplayStatics.GetPlayerCharacter` 0)))
  (remove `/Game/BluePrints/Character/BP_MainCharacter.ED_GetItem` _asbp_main_character (delegate `self.GiveItemToCharacter`))
  (set `/Game/BluePrints/Character/BP_MainCharacter.bCanGetItem` false _asbp_main_character)
  (`KismetSystemLibrary.PrintString` "StopOverlap")
  (`PaperSpriteComponent.SetSpriteColor` (`self.RenderComponent`) (`self.Sprite Color Backup`))
  (`self.RemoveFromGameWidget` (`self.WBP_Riddle2`)))

(fn `UserConstructionScript`
  (`parent.UserConstructionScript`))