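; BP_Regal is an interactable sprite shelf that takes a book from the player's inventory for a riddle.
; Box overlap binds or unbinds the player's get-item dispatcher and tints the sprite or restores its color, removing the widget on exit.
; Interacting looks up the actor's item in DT_Items, removes it from inventory and toggles a lazily created WBP_Riddle1.
; A successful removal fills the widget's first empty slot after a short delay.
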(event `self.GiveItemToCharacter`
  (bind _asbp_main_character (cast `/Game/BluePrints/Character/BP_MainCharacter` (`GameplayStatics.GetPlayerCharacter` 0)))
  (bind _returnvalue (`|GetDataTableRow` "/Game/BluePrints/DataTables/DT_Items.DT_Items" (`.RowName` (break `DataTableRowHandle` (`self.ItemInActor`))))
    (:`then`
      (bind _bremoved (`/Game/BluePrints/Components/Player/BP_InventoryComponents.RemoveItemFromInv` (`/Game/BluePrints/Character/BP_MainCharacter.BP_InventoryComponents` _asbp_main_character) _returnvalue))
      (set `self.bBookRemoved` _bremoved)
      (`self.WBP_Riddle`
        (:`then`
          _)
        (:`else`
          (bind _returnvalue_2 (`|CreateWidget` "/Game/Widgets/Riddle1/WBP_Riddle1.WBP_Riddle1_C"))
          (set `self.WBP_Riddle` _returnvalue_2)))
      (`|ExecutionSequence`
        (:`then_0`
          (if (`self.bBookRemoved`)
            (`KismetSystemLibrary.Delay` 0.2)
            (`/Game/Widgets/Riddle1/WBP_Riddle1.SetInFirstEmpty` (`self.WBP_Riddle`))
            (set `self.bBookRemoved` false)))
        (:`then_1`
          (`self.AddOrRemoveWidget` (`self.WBP_Riddle`)))))))

(event `self.Box.OnComponentBeginOverlap`
  (params (OverlappedComponent :type "PrimitiveComponent Object Reference") (OtherActor :type "Actor Object Reference") (OtherComp :type "PrimitiveComponent Object Reference") (OtherBodyIndex :type Integer) (bFromSweep :type Boolean) (SweepResult :type "HitResult Structure (by ref)"))
  (bind _rendercomponent (`self.RenderComponent`))
  (bind _asbp_main_character (cast `/Game/BluePrints/Character/BP_MainCharacter` (`GameplayStatics.GetPlayerCharacter` 0)))
  (add `/Game/BluePrints/Character/BP_MainCharacter.ED_GetItem` _asbp_main_character (delegate `self.GiveItemToCharacter`))
  (set `/Game/BluePrints/Character/BP_MainCharacter.bCanGetItem` true _asbp_main_character)
  (`KismetSystemLibrary.PrintString` "OverlapInteactActor")
  (set `self.Sprite Color Backup` (`PaperSpriteComponent.SpriteColor` _rendercomponent))
  (`PaperSpriteComponent.SetSpriteColor` _rendercomponent (`self.New Color`)))

(event `self.Box.OnComponentEndOverlap`
  (params (OverlappedComponent :type "PrimitiveComponent Object Reference") (OtherActor :type "Actor Object Reference") (OtherComp :type "PrimitiveComponent Object Reference") (OtherBodyIndex :type Integer))
  (bind _asbp_main_character (cast `/Game/BluePrints/Character/BP_MainCharacter` (`GameplayStatics.GetPlayerCharacter` 0)))
  (remove `/Game/BluePrints/Character/BP_MainCharacter.ED_GetItem` _asbp_main_character (delegate `self.GiveItemToCharacter`))
  (set `/Game/BluePrints/Character/BP_MainCharacter.bCanGetItem` false _asbp_main_character)
  (`KismetSystemLibrary.PrintString` "StopOverlap")
  (`PaperSpriteComponent.SetSpriteColor` (`self.RenderComponent`) (`self.Sprite Color Backup`))
  (`self.RemoveFromGameWidget` (`self.WBP_Riddle`)))

(fn `UserConstructionScript`
  (`parent.UserConstructionScript`))