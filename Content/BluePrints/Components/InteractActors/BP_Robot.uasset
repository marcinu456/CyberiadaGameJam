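; BP_Robot is a sprite-based interactable that completes the robot and ends the game with the credits.
; Box overlap tints the sprite, enables the character's CanGetItem and binds the give-item event to its EDGetItem dispatcher; leaving reverts this.
; The event clears Mask, removes the DT_Items item from inventory, disables collision and swaps to the whole-robot sprite.
; After a delay, it shows the credits widget with UI-only input and hides the HUD.
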(event `self.ReceiveBeginPlay`
  (`parent.ReceiveBeginPlay`))

(event `self.ReceiveTick`
  (params (DeltaSeconds :type "Float (single-precision)"))
  (`parent.ReceiveTick` DeltaSeconds))

(event `self.GiveItemToCharacter`
  (remove `/Game/BluePrints/Character/BP_MainCharacter.ED_GetItem` (stale `self.Box.OnComponentBeginOverlap` _asbp_main_character) (delegate `self.GiveItemToCharacter`))
  (bind _asbp_main_character (cast `/Game/BluePrints/Character/BP_MainCharacter` (`GameplayStatics.GetPlayerCharacter` 0)))
  (set `/Game/BluePrints/Character/BP_MainCharacter.Mask` false _asbp_main_character)
  (bind _returnvalue (`|GetDataTableRow` "/Game/BluePrints/DataTables/DT_Items.DT_Items" (`.RowName` (break `DataTableRowHandle` (`self.ItemInActor`))))
    (:`then`
      (`/Game/BluePrints/Components/Player/BP_InventoryComponents.RemoveItemFromInv` (`/Game/BluePrints/Character/BP_MainCharacter.BP_InventoryComponents` _asbp_main_character) _returnvalue)
      (`PrimitiveComponent.SetCollisionEnabled` (`self.Box`) "NoCollision")
      (`PaperSpriteComponent.SetSprite` (`self.RenderComponent`) "/Game/AssetTextures/Meble/robot_calosc_Sprite.robot_calosc_Sprite")
      (`KismetSystemLibrary.Delay` 3.0)
      (`WidgetBlueprintLibrary.SetInputMode_UIOnlyEx` (`GameplayStatics.GetPlayerController` 0) null)
      (set `PlayerController.bShowMouseCursor` true (`GameplayStatics.GetPlayerController` 0))
      (bind _returnvalue_2 (`|CreateWidget` "/Game/Widgets/Credits/Credits1.Credits1_C"))
      (`UserWidget.AddToViewport` _returnvalue_2 0)
      (bind _asbp_game_hud (cast `/Game/BluePrints/UI/BP_GameHud` (`PlayerController.GetHUD` (`GameplayStatics.GetPlayerController` 0))))
      (`/Game/BluePrints/UI/BP_GameHud.HideHud` _asbp_game_hud))))

(event `self.Box.OnComponentBeginOverlap`
  (params (OverlappedComponent :type "PrimitiveComponent Object Reference") (OtherActor :type "Actor Object Reference") (OtherComp :type "PrimitiveComponent Object Reference") (OtherBodyIndex :type Integer) (bFromSweep :type Boolean) (SweepResult :type "HitResult Structure (by ref)"))
  (bind _rendercomponent (`self.RenderComponent`))
  (bind _asbp_main_character (cast `/Game/BluePrints/Character/BP_MainCharacter` (`GameplayStatics.GetPlayerCharacter` 0)))
  (add `/Game/BluePrints/Character/BP_MainCharacter.ED_GetItem` _asbp_main_character (delegate `self.GiveItemToCharacter`))
  (set `/Game/BluePrints/Character/BP_MainCharacter.bCanGetItem` true _asbp_main_character)
  (`KismetSystemLibrary.PrintString` "OverlapInteactActor")
  (set `self.Sprite Color Backup` (`PaperSpriteComponent.SpriteColor` _rendercomponent))
  (`PaperSpriteComponent.SetSpriteColor` _rendercomponent (`self.New Color`)))

(event `self.Box.OnComponentEndOverlap`
  (params (OverlappedComponent :type "PrimitiveComponent Object Reference") (OtherActor :type "Actor Object Reference") (OtherComp :type "PrimitiveComponent Object Reference") (OtherBodyIndex :type Integer))
  (bind _asbp_main_character (cast `/Game/BluePrints/Character/BP_MainCharacter` (`GameplayStatics.GetPlayerCharacter` 0)))
  (remove `/Game/BluePrints/Character/BP_MainCharacter.ED_GetItem` _asbp_main_character (delegate `self.GiveItemToCharacter`))
  (set `/Game/BluePrints/Character/BP_MainCharacter.bCanGetItem` false _asbp_main_character)
  (`KismetSystemLibrary.PrintString` "StopOverlap")
  (`PaperSpriteComponent.SetSpriteColor` (`self.RenderComponent`) (`self.Sprite Color Backup`)))

(fn `UserConstructionScript`
  (`parent.UserConstructionScript`))