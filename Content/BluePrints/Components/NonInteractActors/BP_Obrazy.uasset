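; BP_Obrazy is a non-interactive world actor whose visual is visible only while the player character's Mask flag is off.
; It caches the player's BP_MainCharacter on BeginPlay, then polls Mask every Tick to hide or show its RenderComponent.
; The visibility change does not propagate to child components.
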(event `self.ReceiveBeginPlay`
  (bind _asbp_main_character (cast `/Game/BluePrints/Character/BP_MainCharacter` (`GameplayStatics.GetPlayerCharacter` 0)))
  (set `self.Main Character` _asbp_main_character))

(event `self.ReceiveTick`
  (params (DeltaSeconds :type "Float (single-precision)"))
  (if (`/Game/BluePrints/Character/BP_MainCharacter.Mask` (`self.Main Character`))
    (`SceneComponent.SetHiddenInGame` (`self.RenderComponent`) true false)
    (else
      (`SceneComponent.SetHiddenInGame` (`self.RenderComponent`) false false))))

(fn `UserConstructionScript`)