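; BP_PolkaSloiki is a non-interactive jar shelf actor that appears once the player character is in the cellar (Piwnica).
; On BeginPlay it caches the BP_MainCharacter reference, hides its RenderComponent and disables collision.
; Tick polls the character's InPiwnica flag and, while true, shows the component and enables query and physics collision.
; Nothing in the Blueprint hides it again afterwards.
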(event `self.ReceiveBeginPlay`
  (bind _asbp_main_character (cast `/Game/BluePrints/Character/BP_MainCharacter` (`GameplayStatics.GetPlayerCharacter` 0)))
  (set `self.MainCharacter` _asbp_main_character)
  (`SceneComponent.SetHiddenInGame` (`self.RenderComponent`) true false)
  (`PrimitiveComponent.SetCollisionEnabled` (`self.RenderComponent`) "NoCollision"))

(event `self.ReceiveTick`
  (params (DeltaSeconds :type "Float (single-precision)"))
  (if (`/Game/BluePrints/Character/BP_MainCharacter.InPiwnica` (`self.MainCharacter`))
    (`SceneComponent.SetHiddenInGame` (`self.RenderComponent`) false false)
    (`PrimitiveComponent.SetCollisionEnabled` (`self.RenderComponent`) "QueryAndPhysics")))

(fn `UserConstructionScript`)