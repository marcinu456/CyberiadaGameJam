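; Player inventory component that holds a fixed-slot item array, tracks the active item and mirrors changes to the HUD inventory widget.
; Adding fills the first "NoneItem" slot, and selecting a slot resolves its full data by scanning the item data table by IDName.
; Removal only succeeds for the active item, resetting its slot to "NoneItem".
; On BeginPlay it populates the widget and selects the first slot; Tick prints the active item's ID on screen.
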(event `self.ReceiveBeginPlay`
  (`self.InitInv`))

(event `self.ReceiveTick`
  (params (DeltaSeconds :type "Float (single-precision)"))
  (`KismetSystemLibrary.PrintString` (`.IDName_6_F3D594CF4D98A2195EE6EF8277EE8A94` (break `/Game/BluePrints/Structures/BPS_ItemInventory` (`self.CurrentActiveItem`))) true false (struct :`G` 0.66 :`B` 1.0 :`A` 1.0) 0.0))

(fn `AddItemToInv`
  (params (NewItem :type "/Game/BluePrints/Structures/BPS_ItemInventory Structure"))
  (bind _inventory (`self.Inventory`))
  (bind _bps_iteminventoryslot (make `/Game/BluePrints/Structures/BPS_ItemInventorySlot` (`.IDName_6_F3D594CF4D98A2195EE6EF8277EE8A94` (break `/Game/BluePrints/Structures/BPS_ItemInventory` NewItem))))
  (for (_array_element _array_index) _inventory
    (if (`KismetStringLibrary.EqualEqual_StrStr` (`.IDName_6_F3D594CF4D98A2195EE6EF8277EE8A94` (break `/Game/BluePrints/Structures/BPS_ItemInventorySlot` _array_element)) "NoneItem")
      (`KismetArrayLibrary.Array_Set` _inventory _array_index _bps_iteminventoryslot)
      (bind _asbp_game_hud (cast `/Game/BluePrints/UI/BP_GameHud` (`PlayerController.GetHUD` (`GameplayStatics.GetPlayerController` 0))))
      (`/Game/Widgets/Game/WBP_Inventory.AddItem` (`/Game/Widgets/Game/WBP_GameInterface.WBP_Inventory` (`/Game/BluePrints/UI/BP_GameHud.GameInterface` _asbp_game_hud)) _bps_iteminventoryslot _array_index)
      (if (== (`self.Current Item Index`) _array_index)
        (`self.SetActiveItemInInv` (`self.Current Item Index`))
        (break)
        (else
          (break))))))

(fn `InitInv`
  (bind _asbp_game_hud (cast `/Game/BluePrints/UI/BP_GameHud` (`PlayerController.GetHUD` (`GameplayStatics.GetPlayerController` 0))))
  (for (_array_element _array_index) (`self.Inventory`)
    (`/Game/Widgets/Game/WBP_Inventory.AddItem` (`/Game/Widgets/Game/WBP_GameInterface.WBP_Inventory` (`/Game/BluePrints/UI/BP_GameHud.GameInterface` _asbp_game_hud)) _array_element _array_index))
  (`self.SetActiveItemInInv` 0))

(fn `RemoveItemFromInv`
  (params (NewItem :type "/Game/BluePrints/Structures/BPS_ItemInventory Structure"))
  (returns (bRemoved :type Boolean))
  (locals (NewLocalVar :type "/Game/BluePrints/Structures/BPS_ItemInventorySlot Structure") (CurrentIndex :type Integer :default 0))
  (bind _inventory (`self.Inventory`))
  (bind _idname (break `/Game/BluePrints/Structures/BPS_ItemInventory` (`self.CurrentActiveItem`)))
  (if (`KismetStringLibrary.EqualEqual_StrStr` _idname (`.IDName_6_F3D594CF4D98A2195EE6EF8277EE8A94` (break `/Game/BluePrints/Structures/BPS_ItemInventory` NewItem)))
    (bind _output_get (set `local.CurrentIndex` (`KismetArrayLibrary.Array_Find` _inventory (make `/Game/BluePrints/Structures/BPS_ItemInventorySlot` _idname))))
    (`KismetArrayLibrary.Array_Set` _inventory _output_get (make `/Game/BluePrints/Structures/BPS_ItemInventorySlot` "NoneItem"))
    (bind _asbp_game_hud (cast `/Game/BluePrints/UI/BP_GameHud` (`PlayerController.GetHUD` (`GameplayStatics.GetPlayerController` 0))))
    (`/Game/Widgets/Game/WBP_Inventory.AddItem` (`/Game/Widgets/Game/WBP_GameInterface.WBP_Inventory` (`/Game/BluePrints/UI/BP_GameHud.GameInterface` _asbp_game_hud)) (`|GetArrayItem` (`self.Inventory`) _output_get) _output_get)
    (set `self.CurrentActiveItem` (make `/Game/BluePrints/Structures/BPS_ItemInventory` "NoneItem" "None" "/Game/Icons/muted_icon.muted_icon"))
    (return true)
    (else
      (return false))))

(fn `SetActiveItemInInv`
  (params (ItemIndex :type Integer))
  (locals (ItemDataTable :type "DataTable Object Reference" :default "/Script/Engine.DataTable'/Game/BluePrints/DataTables/DT_Items.DT_Items'"))
  (set `self.Current Item Index` ItemIndex)
  (bind _outrownames (`DataTableFunctionLibrary.GetDataTableRowNames` (`local.ItemDataTable`)))
  (for _array_element _outrownames
    (bind _returnvalue (`|GetDataTableRow` (`local.ItemDataTable`) _array_element)
      (:`then`
        (if (`KismetStringLibrary.EqualEqual_StrStr` (`.IDName_6_F3D594CF4D98A2195EE6EF8277EE8A94` (break `/Game/BluePrints/Structures/BPS_ItemInventory` _returnvalue)) (`.IDName_6_F3D594CF4D98A2195EE6EF8277EE8A94` (break `/Game/BluePrints/Structures/BPS_ItemInventorySlot` (`|GetArrayItem` (`self.Inventory`) ItemIndex))))
          (set `self.CurrentActiveItem` _returnvalue)
          (bind _asbp_game_hud (cast `/Game/BluePrints/UI/BP_GameHud` (`PlayerController.GetHUD` (`GameplayStatics.GetPlayerController` 0))))
          (`/Game/Widgets/Game/WBP_Inventory.SetCurrentActiveItem` (`/Game/Widgets/Game/WBP_GameInterface.WBP_Inventory` (`/Game/BluePrints/UI/BP_GameHud.GameInterface` _asbp_game_hud)) ItemIndex)
          (break))))))