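; BP_Level is a Paper2D tile map level actor that changes the room's look depending on whether the player character wears a mask.
; Shortly after BeginPlay it casts the player pawn to BP_MainCharacter and caches the reference.
; Every tick it reads that character's Mask flag and sets the render component to either the Pokojx4 tile map or the maskless room variant.
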(event `self.ReceiveBeginPlay`
  (`KismetSystemLibrary.Delay` 0.2)
  (bind _asbp_main_character (cast `/Game/BluePrints/Character/BP_MainCharacter` (`GameplayStatics.GetPlayerCharacter` 0)))
  (set `self.MainCharacter` _asbp_main_character))

(event `self.ReceiveTick`
  (params (DeltaSeconds :type "Float (single-precision)"))
  (bind _maincharacter (`self.MainCharacter`)
    (:`then`
      (if (`/Game/BluePrints/Character/BP_MainCharacter.Mask` _maincharacter)
        (`PaperTileMapComponent.SetTileMap` (`self.RenderComponent`) "/Game/Maps/Textury/TexturyMapy/Pokojx4TileMap.Pokojx4TileMap")
        (else
          (`PaperTileMapComponent.SetTileMap` (`self.RenderComponent`) "/Game/Maps/Textury/TexturyMapy/TM_PokójBezMaski.TM_PokójBezMaski"))))
    (:`else`)))

(fn `UserConstructionScript`)